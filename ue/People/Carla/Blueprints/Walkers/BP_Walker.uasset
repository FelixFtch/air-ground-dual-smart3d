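; CARLA pedestrian walker that dies when a vehicle's skeletal mesh overlaps its death triggers.
; Prop attaches a held mesh and fits a second trigger around it; on impact the prop drops with physics.
; The hit either ragdolls the mesh or, with deterministic ragdolls enabled, simulates the capsule and plays the death animation nearest the collision angle.
; After death, movement stops and Tick gradually reorients the body to face upwards.
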(event `self.PedestrianPropDeathTrigger.OnComponentBeginOverlap`
  (params (OverlappedComponent :type "PrimitiveComponent Object Reference") (OtherActor :type "Actor Object Reference") (OtherComp :type "PrimitiveComponent Object Reference") (OtherBodyIndex :type Integer) (bFromSweep :type Boolean) (SweepResult :type "HitResult Structure (by ref)"))
  (if (and (not (`self.bIsInvincible`)) (`self.bAlive`))
    (`self.HitBySomething` OtherActor OtherComp)))

(event `self.PedestrianDeathTrigger.OnComponentBeginOverlap`
  (params (OverlappedComponent :type "PrimitiveComponent Object Reference") (OtherActor :type "Actor Object Reference") (OtherComp :type "PrimitiveComponent Object Reference") (OtherBodyIndex :type Integer) (bFromSweep :type Boolean) (SweepResult :type "HitResult Structure (by ref)"))
  (if (and (not (`self.bIsInvincible`)) (`self.bAlive`))
    (`self.HitBySomething` OtherActor OtherComp)))

(event `self.ReceiveTick`
  (params (DeltaSeconds :type "Float (single-precision)"))
  (bind _mesh (`self.Mesh`))
  (bind _returnvalue (* DeltaSeconds (`self.DeathOrientationSpeed`)))
  (bind (_x _y) (`KismetMathLibrary.GetAxes` (`SceneComponent.K2_GetComponentRotation` _mesh)))
  (bind (_x_2 _y_2 _z) (`KismetMathLibrary.GetAxes` (`SceneComponent.K2_GetComponentRotation` (`self.CapsuleComponent`))))
  (bind _returnvalue_2 (`KismetMathLibrary.Normal` (`KismetMathLibrary.Cross_VectorVector` _z (0.0 0.0 1.0))))
  (bind _returnvalue_3 (select `bool` (< (`KismetMathLibrary.Vector_DistanceSquared` (0.0 0.0 1.0) (`.Y` (`KismetMathLibrary.GetAxes` (`SceneComponent.K2_GetComponentRotation` (`self.Mesh`))))) 2.0) :`false` (* _returnvalue_2 -1) :`true` _returnvalue_2))
  ;[1 1 1] Set Orientation when the character dies to always face upwards
  (if (not (`self.bAlive`))
    (`SceneComponent.K2_SetWorldRotation` _mesh (`KismetMathLibrary.MakeRotationFromAxes` (`KismetMathLibrary.VLerp` _x (* _returnvalue_3 -1) _returnvalue) (`KismetMathLibrary.VLerp` _y (`KismetMathLibrary.Cross_VectorVector` _returnvalue_3 _z) _returnvalue) _z) false false)))

(fn `GetAnimationFromCollisionAngle`
  (params (CollisionAngle :type "Float (double-precision)"))
  (returns (Animation :type "SingleAnimationPlayData Structure"))
  (locals (ClosestValue :type "Float (double-precision)" :default 10000.0) (ClosestIndex :type Integer))
  (bind _animationmap (`self.AnimationMap`))
  (`|ExecutionSequence`
    (:`then_0`
      ;[1 1 1] Get closest animation to collision angle
      (bind _keys (`BlueprintMapLibrary.Map_Keys` _animationmap))
      (for (_array_element _array_index) _keys
        (bind _returnvalue (`KismetMathLibrary.Abs` (- CollisionAngle _array_element)))
        (if (< _returnvalue (`local.ClosestValue`))
          (set `local.ClosestValue` _returnvalue)
          (set `local.ClosestIndex` _array_index))
        (bind _returnvalue_2 (`KismetMathLibrary.Abs` (- (+ _array_element 360.0) CollisionAngle)))
        (if (< _returnvalue_2 (`local.ClosestValue`))
          (set `local.ClosestValue` _returnvalue_2)
          (set `local.ClosestIndex` _array_index))))
    (:`then_1`
      (bind _keys_2 (`BlueprintMapLibrary.Map_Keys` (`self.AnimationMap`)))
      (return (`BlueprintMapLibrary.Map_Find` _animationmap (`|GetArrayItem` _keys_2 (`local.ClosestIndex`)))))))

(fn `HitByCar`
  (params (CollisionAngle :type "Float (double-precision)"))
  (bind _capsulecomponent (`self.CapsuleComponent`))
  (bind _holdmesh (`self.HoldMesh`))
  (bind _mesh (`self.Mesh`))
  (bind _returnvalue (`CharacterMovementComponent.GetLastUpdateVelocity` (`self.CharacterMovement`)))
  (bind (_returnvalue_bsynchronousmode _returnvalue_bnorenderingmode _returnvalue_bsubstepping _returnvalue_bdeterministicragdolls) (break `EpisodeSettings` (`CarlaEpisode.GetSettings` (`CarlaStatics.GetCurrentEpisode`))))
  (`|ExecutionSequence`
    (:`then_0`
      (if (`KismetSystemLibrary.IsValid` _holdmesh)
        ;[1 1 1] Enable physics in the colided object
        (`SceneComponent.K2_DetachFromComponent` _holdmesh "KeepWorld" "KeepWorld" "KeepWorld" true)
        (`PrimitiveComponent.SetSimulatePhysics` _holdmesh true)
        (`PrimitiveComponent.SetCollisionEnabled` _holdmesh "QueryAndPhysics")))
    (:`then_1`
      (if _returnvalue_bdeterministicragdolls
        ;[1 1 1] Set physics simulation
        (`PrimitiveComponent.SetSimulatePhysics` _capsulecomponent true)
        (`PrimitiveComponent.SetCollisionEnabled` _capsulecomponent "QueryAndPhysics")
        (`PrimitiveComponent.SetCollisionResponseToChannel` (`self.Mesh`) "ECC_Vehicle" "ECR_Ignore")
        (`PrimitiveComponent.SetPhysicsLinearVelocity` _capsulecomponent _returnvalue false "None")
        ;[1 1 1] Play death animation
        (bind _animation (`self.GetAnimationFromCollisionAngle` CollisionAngle))
        (`SkeletalMeshComponent.PlayAnimation` (`self.Mesh`) (break `SingleAnimationPlayData` _animation) false)
        (else
          (`PrimitiveComponent.SetSimulatePhysics` _mesh true)
          (`PrimitiveComponent.SetCollisionEnabled` _mesh "QueryAndPhysics")
          (`PrimitiveComponent.SetPhysicsLinearVelocity` _mesh _returnvalue false "None")))
      (`BoxComponent.SetBoxExtent` (`self.PedestrianDeathTrigger`) (1.0 1.0 1.0) true)
      (`BoxComponent.SetBoxExtent` (`self.PedestrianPropDeathTrigger`) (1.0 1.0 1.0) true)
      (`BoxComponent.SetBoxExtent` (`self.CarStopper`) (20.0 20.0 20.0) true))
    (:`then_2`
      (set `self.bAlive` false)
      (`self.SetActorTickEnabled` true)
      (`CharacterMovementComponent.DisableMovement` (`self.CharacterMovement`)))))

(fn `HitBySomething`
  (params (HitByActor :type "Actor Object Reference") (HitByComponent :type "ActorComponent Object Reference"))
  (locals (CollisionAngle :type "Float (double-precision)"))
  (bind (_returnvalue_x _returnvalue_y) (`KismetMathLibrary.BreakVector2D` (`KismetMathLibrary.NormalSafe2D` (`KismetMathLibrary.Conv_VectorToVector2D` (`KismetMathLibrary.TransformLocation` (`KismetMathLibrary.InvertTransform` (`self.GetTransform`)) (`self.K2_GetActorLocation` HitByActor))))))
  (bind _returnvalue (`KismetMathLibrary.DegAtan2` _returnvalue_y _returnvalue_x))
  ;[1 1 1] If it's a car
  (cast `/Game/Carla/Blueprints/Vehicles/BaseVehiclePawn` HitByActor)
  (cast `SkeletalMeshComponent` HitByComponent)
  ;[1 1 1] Convert [-180,180] angle range to [0,360]
  (if (> _returnvalue 0.0)
    (`self.HitByCar` _returnvalue)
    (else
      (`self.HitByCar` (`KismetMathLibrary.MapRangeClamped` _returnvalue -180.0 0.0 180.0 360.0)))))

(fn `IKFootTrace`
  (params (InSocketName :type Name) (TraceDistance :type "Float (double-precision)"))
  (returns (`Ik Offset` :type "Float (double-precision)"))
  (bind _z (.z (`self.K2_GetActorLocation`)))
  (bind _x (.x (`SceneComponent.GetSocketLocation` (`self.Mesh`) InSocketName)))
  (bind _y (.y (`SceneComponent.GetSocketLocation` (`self.Mesh`) InSocketName)))
  (bind _returnvalue (`KismetMathLibrary.MakeVector` _x _y (- _z TraceDistance)))
  (bind (_outhit _returnvalue_2) (`KismetSystemLibrary.LineTraceSingle` :`Start` (`KismetMathLibrary.MakeVector` _x _y _z) :`End` _returnvalue :`TraceChannel` "TraceTypeQuery1" :`bTraceComplex` true :`DrawDebugType` "Persistent"))
  (return (`KismetMathLibrary.SelectFloat` (/ (`KismetMathLibrary.VSize` (- _returnvalue (`.Location` (`GameplayStatics.BreakHitResult` _outhit)))) (`self.IkScale`)) 0.0 _returnvalue_2)))

(fn `Prop`
  (params (`Prop to place` :type "StaticMesh Object Reference") (SocketName :type Name) (RelativeTransform :type "Transform Structure"))
  (returns (Mesh :type "SkeletalMeshComponent Object Reference") (`Prop to place1` :type "StaticMesh Object Reference") (`PropComponent+` :type "StaticMeshComponent Object Reference"))
  (bind _returnvalue (`StaticMesh.GetBoundingBox` `Prop to place`))
  (bind _pedestrianpropdeathtrigger (`self.PedestrianPropDeathTrigger`))
  (bind _holdmesh (`self.HoldMesh`))
  (bind _returnvalue_2 (/ (- (.z (`.Max` (break `Box` _returnvalue))) (.z (break `Box` _returnvalue))) 2.0))
  (set `self.HoldsProp` true)
  (`|ExecutionSequence`
    (:`then_0`
      ;[1 1 1] Add Component
      (bind _returnvalue_3 (`AddComponent|NODE_AddStaticMeshComponent-11` :`RelativeTransform` RelativeTransform))
      (set `self.HoldMesh` _returnvalue_3)
      (`StaticMeshComponent.SetStaticMesh` _holdmesh `Prop to place`)
      (`SceneComponent.K2_AttachToComponent` _holdmesh (`self.Mesh`) SocketName "KeepRelative" "KeepRelative" "KeepRelative" true)
      (`PrimitiveComponent.SetCollisionEnabled` _holdmesh "NoCollision")
      (bind _ascarla_game_instance (cast `CarlaGameInstance` (`GameplayStatics.GetGameInstance`)))
      (`CarlaGameInstance.GetCARLASettings` _ascarla_game_instance)
      (`PrimitiveComponent.SetCullDistance` _holdmesh 0.0))
    (:`then_1`
      ;[1 1 1] Extend Carcrash box
      (`SceneComponent.K2_AttachToComponent` _pedestrianpropdeathtrigger _holdmesh "None" "KeepRelative" "KeepRelative" "KeepRelative" true)
      (`BoxComponent.SetBoxExtent` _pedestrianpropdeathtrigger (`KismetMathLibrary.MakeVector` (+ (/ (- (.x (`.Max` (break `Box` _returnvalue))) (.x (break `Box` _returnvalue))) 2.0) 10.0) (+ (/ (- (.y (`.Max` (break `Box` _returnvalue))) (.y (break `Box` _returnvalue))) 2.0) 10.0) (+ _returnvalue_2 10.0)) true)
      (`SceneComponent.K2_SetRelativeTransform` _pedestrianpropdeathtrigger (`KismetMathLibrary.MakeTransform` (`KismetMathLibrary.MakeVector` 0.0 0.0 (- 1.0 _returnvalue_2))) true false))
    (:`then_2`)
    (:`then_3`
      (return (`self.Mesh`) `Prop to place` _holdmesh))))

(fn `UserConstructionScript`
  (locals (PreviousAnim :type "AnimInstance Class Reference")))