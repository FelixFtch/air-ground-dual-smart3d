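; WalkerSelector is a Carla actor Blueprint that assembles a pedestrian walker variant from gender, body type and sleeve-length settings.
; GenerateWalker uses nested switches to pick one body from Bodies and a matching shirt from ShirtMesh, storing the pair in CurrentWalker.
; It then spawns both as separate, unattached actors at the root's world location via the editor-style SpawnActorFromObject.
; The event graph and construction script are empty.
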(fn `GenerateWalker`
  (bind _bodytype (`self.BodyType`))
  (bind _shirttype (`self.ShirtType`))
  (bind _returnvalue (`SceneComponent.K2_GetComponentLocation` (`self.DefaultSceneRoot`)))
  (switch `/Game/Carla/Blueprints/Walkers/WalkerGenre` (`self.Genre`)
    (:`NewEnumerator0`
      (switch `/Game/Carla/Blueprints/Walkers/WalkerBodyType` _bodytype
        (:`NewEnumerator0`
          (set `self.Current Walker Body` (`|GetArrayItem` (`self.Bodies`)))
          (switch `/Game/Carla/Blueprints/Walkers/ShirtType` _shirttype
            (:`NewEnumerator0`
              (set `self.Current Walker Shirt` (`|GetArrayItem` (`self.ShirtMesh`))))
            (:`NewEnumerator1`
              (set `self.Current Walker Shirt` (`|GetArrayItem` (`self.ShirtMesh`) 1)))))
        (:`NewEnumerator1`
          (set `self.Current Walker Body` (`|GetArrayItem` (`self.Bodies`) 1))
          (switch `/Game/Carla/Blueprints/Walkers/ShirtType` _shirttype
            (:`NewEnumerator0`
              (set `self.Current Walker Shirt` (`|GetArrayItem` (`self.ShirtMesh`) 2)))
            (:`NewEnumerator1`
              (set `self.Current Walker Shirt` (`|GetArrayItem` (`self.ShirtMesh`) 3)))))))
    (:`NewEnumerator1`
      (switch `/Game/Carla/Blueprints/Walkers/WalkerBodyType` _bodytype
        (:`NewEnumerator0`
          (set `self.Current Walker Body` (`|GetArrayItem` (`self.Bodies`) 2))
          (switch `/Game/Carla/Blueprints/Walkers/ShirtType` _shirttype
            (:`NewEnumerator0`
              (set `self.Current Walker Shirt` (`|GetArrayItem` (`self.ShirtMesh`) 4)))
            (:`NewEnumerator1`
              (set `self.Current Walker Shirt` (`|GetArrayItem` (`self.ShirtMesh`) 5)))))
        (:`NewEnumerator1`
          (set `self.Current Walker Body` (`|GetArrayItem` (`self.Bodies`) 3))
          (switch `/Game/Carla/Blueprints/Walkers/ShirtType` _shirttype
            (:`NewEnumerator0`
              (set `self.Current Walker Shirt` (`|GetArrayItem` (`self.ShirtMesh`) 6)))
            (:`NewEnumerator1`
              (set `self.Current Walker Shirt` (`|GetArrayItem` (`self.ShirtMesh`) 7))))))))
  (set `self.CurrentWalker` (make `/Game/Carla/Blueprints/Walkers/Walker` (`self.Current Walker Body`) (`self.Current Walker Shirt`)))
  (`EditorLevelLibrary.SpawnActorFromObject` (`self.Current Walker Body`) _returnvalue)
  (`EditorLevelLibrary.SpawnActorFromObject` (`self.Current Walker Shirt`) _returnvalue))

(fn `UserConstructionScript`)