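; BP_WalkerFactory is a pedestrian factory that finishes setting up spawned walker actors and keeps their parameter definitions.
; PostProcessWalker gives a spawned pawn the walker AI controller, then sets BP_Walker invincibility from the "is_invincible" variation attribute, defaulting to true.
; It reports failure for anything that is not a BP_Walker.
; Two helper functions save and load the walker parameters array through WalkerParameters.json.
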(event `self.ReceiveBeginPlay`)

(fn `Load Pedestrian Parameters from Json`
  (bind _outwalkerparamsarray (`self.LoadWalkerParametersArrayFromFile` "WalkerParameters.json"))
  (set `self.WalkersParams` _outwalkerparamsarray))

(fn `PostProcessWalker`
  (params (SpawnedActor :type "Actor Object Reference") (WalkerParams :type "ActorDescription Structure (by ref)"))
  (returns (ReturnValue :type Boolean))
  (bind _aspawn (cast `Pawn` SpawnedActor)
    (:`then`
      (set `Pawn.AIControllerClass` "/Script/Carla.WalkerController" _aspawn)
      (`Pawn.SpawnDefaultController` _aspawn)
      (bind _asbp_walker (cast `/Game/Carla/Blueprints/Walkers/BP_Walker` SpawnedActor)
        (:`then`
          (bind _returnvalue (`ActorBlueprintFunctionLibrary.RetrieveActorAttributeToBool` "is_invincible" (`.Variations` (break `ActorDescription` WalkerParams)) true))
          (set `/Game/Carla/Blueprints/Walkers/BP_Walker.bIsInvincible` _returnvalue _asbp_walker)
          (return true))
        (:`CastFailed`
          (return false))))
    (:`CastFailed`
      (return false))))

(fn `UserConstructionScript`)

(fn `Write Pedestrian Parameters To Json`
  (`self.SaveWalkerParametersArrayToFile` (`self.WalkersParams`) "WalkerParameters.json"))